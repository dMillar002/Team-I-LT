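; Door Blueprint with Top and Bottom parts that slide between open and closed, apparently driven by a button or pressure switch.
; Each SwitchOn&Off event flips a FlipFlop that alternately plays and reverses a Timeline.
; The Timeline lerps both parts' relative locations between their Current and New vectors, which are not assigned in these graphs.
; An unconnected leftover DoorTimeline chain moves only Top along Z.
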(event `SwitchOn&Off`
  (`/Engine/EditorBlueprintResources/StandardMacros.FlipFlop`
    (:`A`
      (bind (_direction _slide) (`Timeline|Timeline` :!label _label)
        (:`Update`
          (`SceneComponent.K2_SetRelativeLocation` (`self.Top`) (`KismetMathLibrary.VLerp` (`self.CurrentTop`) (`self.NewTop`) _slide) false false)
          (`SceneComponent.K2_SetRelativeLocation` (`self.Bottom`) (`KismetMathLibrary.VLerp` (`self.Current Bottom`) (`self.NewBottom`) _slide) false false))))
    (:`B`
      (goto _label :!via `Reverse`))))

(fn `UserConstructionScript`)