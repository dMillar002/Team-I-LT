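; Test automatic door actor whose left and right panels slide open when BP_ThirdPersonCharacter overlaps AutoDoorCollisionBox.
; A timeline lerps both panels, reversing when the character ends overlap with LeftAutoDoor, which also disables input.
; A gated IA_Interact path plays a press animation on LeftAutoDoor, then flip-flops a timeline that rotates the actor open or closed.
; The logic to open and close that gate is disconnected.
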(event `EnhancedInput|/Game/ThirdPerson/Input/Actions/IA_Interact`
  (params (ActionValue :type Boolean) (ElapsedSeconds :type "Float (double-precision)") (TriggeredSeconds :type "Float (double-precision)") (InputAction :type "InputAction Object Reference" :default "/Game/ThirdPerson/Input/Actions/IA_Interact.IA_Interact"))
  (:`Triggered`
    (`/Engine/EditorBlueprintResources/StandardMacros.Gate` true
      (:`Exit`
        ;[1 1 1] Play Button Animation
        (bind (_direction _open_door_button_track) (`Timeline|Timeline` :!via `PlayFromStart`)
          (:`Update`
            (`SceneComponent.K2_SetRelativeLocation` (`self.LeftAutoDoor`) (`KismetMathLibrary.VLerp` (`self.Button_Out`) (`self.Button_In`) _open_door_button_track) false false))
          (:`Finished`
            (`/Engine/EditorBlueprintResources/StandardMacros.FlipFlop`
              (:`A`
                (bind (_direction_2 _opendoortrack) (`Timeline|Door_Button_Timeline` :!label _label)
                  (:`Update`
                    (`self.K2_SetActorRotation` self (`KismetMathLibrary.MakeRotator` 0.0 0.0 (`KismetMathLibrary.Lerp` (`self.ClosedDoorAngle`) (`self.OpenDoorAngle`) _opendoortrack)) false))))
              (:`B`
                (goto _label :!via `Reverse`)))))))))

(event `self.AutoDoorCollisionBox.OnComponentBeginOverlap`
  (params (OverlappedComponent :type "PrimitiveComponent Object Reference") (OtherActor :type "Actor Object Reference") (OtherComp :type "PrimitiveComponent Object Reference") (OtherBodyIndex :type Integer) (bFromSweep :type Boolean) (SweepResult :type "HitResult Structure (by ref)"))
  (cast `/Game/ThirdPerson/Blueprints/BP_ThirdPersonCharacter` OtherActor)
  ;[0 0.2865 0.1791] Plays Door Timeline
  (bind (_direction _openautodoortrack) (`Timeline|AutoDoorTimeline` :!label _label_2)
    (:`Update`
      (`SceneComponent.K2_SetRelativeLocation` (`self.LeftAutoDoor`) (`KismetMathLibrary.VLerp` (`self.CurrentLeft`) (`self.NewLeft`) _openautodoortrack) false false)
      (`SceneComponent.K2_SetRelativeLocation` (`self.RightAutoDoor`) (`KismetMathLibrary.VLerp` (`self.CurrentRight`) (`self.NewRight`) _openautodoortrack) false false))))

(event `self.LeftAutoDoor.OnComponentEndOverlap`
  (params (OverlappedComponent :type "PrimitiveComponent Object Reference") (OtherActor :type "Actor Object Reference") (OtherComp :type "PrimitiveComponent Object Reference") (OtherBodyIndex :type Integer))
  (cast `/Game/ThirdPerson/Blueprints/BP_ThirdPersonCharacter` OtherActor)
  (`self.DisableInput` (`GameplayStatics.GetPlayerController` 0))
  (goto _label_2 :!via `Reverse`))

(fn `UserConstructionScript`)